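; Bullet projectile actor that damages targets it passes through and leaves impact effects on what it hits.
; Overlapping IDamagable actors take random damage drawn from a shared penetration pool, plus gibs; the bullet dies when that pool is overspent.
; Box hits spawn sparks, a randomized normal-aligned decal attached to the struck actor and a pitch-varied sound, destroying the bullet.
; GenerateHeat, not called here, adds heat to the shooter's equipped weapon.
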(event OnComponentHit(Box)
  (params (OtherActor :type Actor%20Object%20Reference) (OtherComp :type Primitive%20Component%20Object%20Reference) (NormalImpulse :type Vector) (Hit :type Hit%20Result%20Structure%20%28by%20ref%29))
  (bind (_bblockinghit _binitialoverlap _time _location _impactpoint _normal _impactnormal) (Collision|BreakHitResult Hit))
  (bind _returnvalue (Math|Random|RandomFloatinRange 4e+01 6e+01))
  (bind _returnvalue_2 (Math|Conversions|RotationFromXVector _impactnormal))
  (bind (_roll _pitch _yaw) (Math|Rotator|BreakRotator _returnvalue_2))
  ;[1 1 1] OnHit
  (Utilities|FlowControl|Sequence
    (:then_0
      (Effects|SpawnEmitteratLocation "/Game/Effects/Bullet_spark.Bullet_spark" _location)
      (bind _returnvalue_3 (Rendering|Decal|SpawnDecalatLocation "/Game/Materials/Decal2_Mat.Decal2_Mat" (Math|Vector|MakeVector 1e+01 _returnvalue _returnvalue) _impactpoint (Math|Rotator|MakeRotator (Math|Random|RandomFloatinRange -1.8e+02 1.8e+02) _pitch _yaw) 999.0))
      (Class|SceneComponent|Attachto _returnvalue_3 (VehicleSound|GetRootComponent OtherActor) "None" "KeepWorldPosition" true)
      (Actor|DestroyActor)
      (bind _returnvalue_4 (Audio|SpawnSoundatLocation "/Game/Sounds/hit_concrete_04.hit_concrete_04" _impactpoint))
      (Audio|Components|Audio|SetPitchMultiplier _returnvalue_4 (Math|Random|RandomFloatinRange 0.7 1.2)))))

(event OnComponentBeginOverlap(Box)
  (params (OtherActor :type Actor%20Object%20Reference) (OtherComp :type Primitive%20Component%20Object%20Reference) (OtherBodyIndex :type Integer) (bFromSweep :type Boolean) (SweepResult :type Hit%20Result%20Structure%20%28by%20ref%29))
  (if (Utilities|DoesObjectImplementInterface OtherActor "/Game/BluePrints/iDamagable.iDamagable_C")
    (bind _output_get (Variables|Default|SetDamageRolled (Math|Random|RandomFloatinRange (Variables|Default|GetMinDamage) (Variables|Default|GetMaxDamagePerPenetration))))
    (Variables|Default|SetMaxTotalDamage%28bullet%20health%29 (- (Variables|Default|GetMaxTotalDamage%28bullet%20health%29) _output_get))
    (if (< (Variables|Default|GetMaxTotalDamage%28bullet%20health%29) 0.0)
      (Class|IDamagable|ChangeHealth(Message) OtherActor (* (+ _output_get (Variables|Default|GetMaxTotalDamage%28bullet%20health%29)) -1.0))
      (Actor|DestroyActor)
      (else
        (Class|IDamagable|ChangeHealth(Message) OtherActor (* _output_get -1.0))))
    (Class|IDamagable|SpawnGibsatHit(Message) OtherActor 3 5 "0, 0, 0")))

(event EventBeginPlay)

(event EventActorBeginOverlap
  (params (OtherActor :type Actor%20Object%20Reference)))

(event EventTick
  (params (DeltaSeconds :type Float%20%28single-precision%29)))

(fn ConstructionScript)

(fn GenerateHeat
  (bind _astop_down_character (Utilities|Casting|CastToTopDownCharacter (Variables|Default|GetShotByThis)))
  (bind _asweapon_item (Utilities|Casting|CastToWeapon_Item (Variables|/Game/BluePrints/TopDownCharacter.TopDownCharacter_C|GetEquippedItem _astop_down_character)))
  (Variables|/Game/BluePrints/Weapon_Item.Weapon_Item_C|SetHeatSinkPool _asweapon_item (+ (Variables|/Game/BluePrints/Weapon_Item.Weapon_Item_C|GetHeatSinkPool _asweapon_item) (Variables|Default|GetHeatGeneration))))