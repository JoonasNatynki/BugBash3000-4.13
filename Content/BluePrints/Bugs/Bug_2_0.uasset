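; Bug enemy character with randomized walk speed, health, and gory hit and death effects.
; ChangeHealth only adjusts health; SpawnGibsatHit spawns impulse-launched gibs, blood particles and an attached decal, then destroys the bug if health is depleted.
; Destruction reuses the gib loop, adds persistent gibs and spawns a corpse, with DoN nodes capping the loops.
; Sight and Tick handlers do nothing, and blackboard targeting code is disconnected.
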(event OnSeePawn(BugSenses)
  (params (Pawn :type Pawn%20Object%20Reference)))

(event EventSpawnGibsatHit
  (params (minCount :type Integer) (maxCount :type Integer) (Impulse%20Normal :type Vector))
  (Utilities|FlowControl|Sequence
    (:then_0
      ;[1 1 1] Spawn gibs at death for n amount
      (Utilities|FlowControl|DoN (Math|Random|RandomIntegerinRange 1 3) :!label _label
        (:Exit
          (bind _returnvalue (Game|SpawnActorfromClass "/Game/BluePrints/Bugs/Bug_1_Gibs/Bug_Gib_1.Bug_Gib_1_C" (Math|Conversions|ToTransform(Vector) (+ (Transformation|GetActorLocation) (Math|Vector|MakeVector (Math|Random|RandomFloatinRange -25.0 25.0) (Math|Random|RandomFloatinRange -25.0 25.0) (Math|Random|RandomFloatinRange -25.0 25.0)))) "AdjustIfPossibleButAlwaysSpawn" 0 0))
          (Physics|AddRadialImpulse (Variables|/Game/BluePrints/Bugs/Bug_1_Gibs/Bug_Gib_1.Bug_Gib_1_C|GetCollision_Box _returnvalue) (Transformation|GetActorLocation) 1e+02 3e+03 "RIF_Constant" false)
          (goto _label))))
    (:then_1
      (Effects|SpawnEmitteratLocation "/Game/Effects/Blood_Splah.Blood_Splah" (Transformation|GetActorLocation))
      (Class|GameplayStatics|SpawnDecalAttached "/Game/Materials/blood_spatter_1.blood_spatter_1" "50.000000,50.000000,50.000000" (Variables|Character|GetMesh self) "" "0, 0,0.000000" "0, 0, 0" "KeepRelativeOffset" 3e+01)
      ;[1 1 1] is dead?
      (if (<= (Variables|Default|GetHealth) 0.0)
        (Variables|Default|SetIsDead? true)
        (Actor|DestroyActor)))))

(event EventBeginPlay
  (Variables|/Script/Engine.CharacterMovementComponent|SetMaxWalkSpeed (Variables|Character|GetCharacterMovement) (Math|Random|RandomFloatinRange 5e+02 7e+02)))

(event EventActorBeginOverlap
  (params (OtherActor :type Actor%20Object%20Reference)))

(event EventTick
  (params (DeltaSeconds :type Float%20%28single-precision%29))
  (if (AI|Components|NavMovement|IsMovingonGround (Variables|Character|GetCharacterMovement))
    _))

(event EventChangeHealth
  (params (amount :type Float%20%28single-precision%29))
  (Variables|Default|SetHealth (+ (Variables|Default|GetHealth) amount)))

(event EventDestroyed
  (bind _returnvalue (Transformation|GetActorLocation))
  (bind _returnvalue_2 (Math|Random|RandomFloatinRange -25.0 25.0))
  (bind _returnvalue_3 (Math|Random|RandomFloatinRange -25.0 25.0))
  (bind _returnvalue_4 (Math|Random|RandomFloatinRange -25.0 25.0))
  (bind _returnvalue_5 (Math|Vector|MakeVector _returnvalue_2 _returnvalue_3 _returnvalue_4))
  (bind _returnvalue_6 (+ _returnvalue _returnvalue_5))
  (bind _returnvalue_7 (Math|Conversions|ToTransform(Vector) _returnvalue_6))
  ;[1 1 1] Spawn gibs at death for n amount
  (Utilities|FlowControl|Sequence
    (:then_0
      (Utilities|FlowControl|DoN (Math|Random|RandomIntegerinRange 1 3) :!label _label
        (:Exit
          (bind _returnvalue_8 (Game|SpawnActorfromClass "/Game/BluePrints/Bugs/Bug_1_Gibs/Bug_Gib_1.Bug_Gib_1_C" _returnvalue_7 "AdjustIfPossibleButAlwaysSpawn" 0 0))
          (Physics|AddRadialImpulse (Variables|/Game/BluePrints/Bugs/Bug_1_Gibs/Bug_Gib_1.Bug_Gib_1_C|GetCollision_Box _returnvalue_8) (Transformation|GetActorLocation) 1e+02 3e+03 "RIF_Constant" false)
          (goto _label))))
    (:then_1
      (bind _returnvalue_9 (Game|SpawnActorfromClass "/Game/BluePrints/Bugs/Bug_1_Gibs/Bug_Gib_Persistent.Bug_Gib_Persistent_C" _returnvalue_7 "AdjustIfPossibleButAlwaysSpawn" 0 0 :!label _label_2)) ; permanent gibs
      (Physics|AddRadialImpulse (Variables|/Game/BluePrints/Bugs/Bug_1_Gibs/Bug_Gib_Persistent.Bug_Gib_Persistent_C|GetCollision_Box _returnvalue_9) (Transformation|GetActorLocation) 1e+02 2e+03 "RIF_Constant" false)
      (Utilities|FlowControl|DoN (Math|Random|RandomIntegerinRange 3 5)
        (:Exit
          (goto _label_2))))
    (:then_2
      (Game|SpawnActorfromClass "/Game/BluePrints/Bugs/Bug_1_Gibs/Bug_2_Corpse.Bug_2_Corpse_C" (Math|Conversions|ToTransform(Vector) (+ _returnvalue "0, 0,-100.000000")) "AlwaysSpawn" 0 0))))

(fn ConstructionScript)