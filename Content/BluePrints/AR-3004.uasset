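; AR-3004 is a pickup weapon for the top-down character that attaches to its weapon socket on overlap.
; Tick aims ShootPoint at the character's AimPosition, adding random spread proportional to movement speed.
; Trigger pulls spawn heat-generating bullets with muzzle effects and randomly pitched sounds, looping through a retriggerable delay for automatic fire.
; Tick also cools the heat pool, blocking fire with steam and sound on overheat until it drops below a cutoff.
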(event EventBeginPlay)

(event Collision|EventActorBeginOverlap
  (params (OtherActor :type Actor%20Object%20Reference))
  ;[1 1 1] EUIQPPING ITEM AND PICKUP
  (bind _astop_down_character (Utilities|Casting|CastToTopDownCharacter OtherActor))
  (Variables|Default|SetIsEquipped? true)
  (Physics|SetSimulatePhysics (Variables|Default|GetWeapon_Mesh) false)
  (Class|Actor|AttachRootComponentto (Variables|/Script/Engine.Character|GetMesh _astop_down_character) "weapon_socket" "SnapToTargetIncludingScale" false)
  (bind _astop_down_character_2 (Utilities|Casting|CastToTopDownCharacter OtherActor))
  (Variables|/Game/BluePrints/TopDownCharacter.TopDownCharacter_C|SetEquippedItem _astop_down_character_2 self)
  (Variables|Default|SetEquippedBy _astop_down_character_2))

(event EventTick
  (params (DeltaSeconds :type Float%20%28single-precision%29))
  (bind _shoot_point (Variables|Default|GetShoot_Point))
  (bind _shoot_point_2 (Variables|Default|GetShoot_Point))
  ;[1 1 1] If the item is equipped, disable physics simulation and aim shootPoint towards AimPosition
  (bind _astop_down_character (Utilities|Casting|CastToTopDownCharacter (Variables|Default|GetEquippedBy)))
  (Transformation|SetWorldRotation _shoot_point_2 (Math|Rotator|FindLookatRotation (Transformation|GetWorldLocation _shoot_point_2) (Math|Vector|MakeVector (+ (.X (Math|Vector|BreakVector (.Location (Collision|BreakHitResult (Variables|/Game/BluePrints/TopDownCharacter.TopDownCharacter_C|GetAim_Position _astop_down_character))))) (* (Math|Random|RandomFloatinRange (* (Math|Vector|VectorLength (Transformation|GetVelocity _astop_down_character)) -1.0) (Math|Vector|VectorLength (Transformation|GetVelocity _astop_down_character))) 0.35)) (+ (.Y (Math|Vector|BreakVector (.Location (Collision|BreakHitResult (Variables|/Game/BluePrints/TopDownCharacter.TopDownCharacter_C|GetAim_Position _astop_down_character))))) (* (Math|Random|RandomFloatinRange (* (Math|Vector|VectorLength (Transformation|GetVelocity _astop_down_character)) -1.0) (Math|Vector|VectorLength (Transformation|GetVelocity _astop_down_character))) 0.35)) (+ (.Z (Math|Vector|BreakVector (.Location (Collision|BreakHitResult (Variables|/Game/BluePrints/TopDownCharacter.TopDownCharacter_C|GetAim_Position _astop_down_character))))) (* (Math|Random|RandomFloatinRange (* (Math|Vector|VectorLength (Transformation|GetVelocity _astop_down_character)) -1.0) (Math|Vector|VectorLength (Transformation|GetVelocity _astop_down_character))) 0.35)))) false false)
  ;[1 1 1] overheat, sounds and effects
  (Variables|Default|SetHeatSinkPool (Math|Float|Clamp(Float) (- (Variables|Default|GetHeatSinkPool) (* (Variables|Default|GetCoolingRate) DeltaSeconds)) 0.0 99999.0))
  (if (and (Variables|Default|GetCanFire) (>= (Variables|Default|GetHeatSinkPool) (Variables|Default|GetMaxFunctioningHeat)))
    (Variables|Default|SetCanFire false)
    (bind _returnvalue (Effects|SpawnEmitterAttached "/Game/Effects/OverHeat_Steam.OverHeat_Steam" (Variables|Default|GetShoot_Point) "None" "0,0.000000, 0"))
    (Variables|Default|SetOverHeat_Steam _returnvalue)
    (Audio|SpawnSoundAttached "/Game/Sounds/OverHeat_1.OverHeat_1" _shoot_point)
    (bind _returnvalue_2 (Audio|SpawnSoundAttached "/Game/Sounds/OverHeat_Loop.OverHeat_Loop" _shoot_point))
    (Variables|Default|SetOverHeat_Sound_Loop _returnvalue_2)
    (elif (and (< (Variables|Default|GetHeatSinkPool) (Variables|Default|GetHeatCutOffPoint)) (not (Variables|Default|GetCanFire)))
      (Variables|Default|SetCanFire true)
      (Components|Activation|Deactivate (Variables|Default|GetOverHeat_Steam))
      (Audio|Components|Audio|AdjustVolume (Variables|Default|GetOverHeat_Sound_Loop) 1.0 0.0 :!class /Script/Engine.AudioComponent)
      (Utilities|FlowControl|Delay 1.0)
      (Components|Activation|Deactivate (Variables|Default|GetOverHeat_Sound_Loop)))))

(event EventTriggerPulled
  (bind _shoot_point (Variables|Default|GetShoot_Point))
  (bind _canfire (Variables|Default|GetCanFire))
  (bind _returnvalue (Transformation|GetWorldLocation _shoot_point))
  ;[1 1 1] FIRE EVENT
  (Variables|Default|SetTriggerDown true)
  (if _canfire
    (bind _returnvalue_2 (Game|SpawnActorfromClass "/Game/BluePrints/Bullet_1.Bullet_1_C" (Transformation|GetWorldTransform (Variables|Default|GetShoot_Point)) "Undefined" 0 0 :!label _label))
    (Variables|/Game/BluePrints/Bullet_1.Bullet_1_C|SetShotByThis _returnvalue_2 (Variables|Default|GetEquippedBy))
    (Default|GenerateHeat _returnvalue_2)
    (Collision|SetCollisionEnabled (Variables|Default|GetWeapon_Mesh) "NoCollision")
    ;;[1 1 1] Particle effects
    (Effects|SpawnEmitteratLocation "/Game/Effects/Muzzle_Flash.Muzzle_Flash" _returnvalue)
    (Effects|SpawnEmitteratLocation "/Game/Effects/Muzzle_Smoke.Muzzle_Smoke" _returnvalue (Transformation|GetActorRotation))
    ;;[1 1 1] Sound effects
    (bind _returnvalue_3 (Audio|SpawnSoundatLocation "/Game/Sounds/Explode_31.Explode_31" _returnvalue))
    (bind _returnvalue_4 (Audio|SpawnSoundatLocation "/Game/Sounds/Muzzle_Explosion_short.Muzzle_Explosion_short" _returnvalue))
    (Audio|Components|Audio|SetPitchMultiplier _returnvalue_4 (Math|Random|RandomFloatinRange 0.8 1.5))
    (Utilities|FlowControl|RetriggerableDelay (Variables|Default|GetFireRate))
    (if (Math|Boolean|ANDBoolean (Variables|Default|GetTriggerDown) _canfire (Variables|Default|GetIsAutoFire?))
      (goto _label))))

(event EventTriggerReleased
  ;[1 1 1] FIRE EVENT
  (Variables|Default|SetTriggerDown false))

(fn ConstructionScript)